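; BP_Ceiling is a paintable ceiling piece for the renovation game, with optional top and bottom meshes toggled in the construction script.
; Interface focus stores the focus state and outlines both meshes when the player holds Tool_04, the brush.
; While focused, a Delay-throttled Tick calls Paint per side, applying the player's current paint material and awarding XP if the player overlaps that side's box and is using paint.
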(event EventInterfaceToggleFocus
  (params (Focus :type Boolean))
  ;[0.05098 0.05098 0.05098] Interaction outline
  (Variables|Interaction|SetFocus Focus)
  ;;[0.1255 0.1255 0.1255] If the player has the brush in his hands
  (if (== (Variables|/Game/RenovationSimulator/Demo/Player/FirstPerson/Blueprints/BP_FirstPersonCharacter.BP_FirstPersonCharacter_C|GetCurrent_Tool (Variables|Player|GetPlayer)) "Tool_04")
    (Rendering|SetRenderCustomDepth (Variables|Default|GetCeiling_Top) (Variables|Interaction|GetFocus))
    (Rendering|SetRenderCustomDepth (Variables|Default|GetCeiling_Bottom) (Variables|Interaction|GetFocus))))

(event EventBeginPlay
  (bind _returnvalue (Game|GetPlayerCharacter 0))
  ;[0.05098 0.05098 0.05098] Initialization
  (bind _asbp_first_person_character (Utilities|Casting|CastToBP_FirstPersonCharacter _returnvalue)
    (:then
      (Variables|Player|SetPlayer _asbp_first_person_character))
    (:CastFailed
      (bind _asvrpawn (Utilities|Casting|CastToVRPawn _returnvalue))
      (Variables|Default|SetNewVar _asvrpawn)))
  (bind _aswbp_interaction_input (Utilities|Casting|CastToWBP_Interaction_Input (UserInterface|GetUserWidgetObject (Variables|Default|GetWidget))))
  (Variables|/Game/RenovationSimulator/Blueprints/Widgets/Childs/WBP_Interaction_Input.WBP_Interaction_Input_C|SetAction _aswbp_interaction_input ""))

(event EventTick
  (params (DeltaSeconds :type Float%20%28single-precision%29))
  ;[0.05098 0.05098 0.05098] Paint
  (Utilities|FlowControl|Delay 0.5)
  (if (Variables|Interaction|GetFocus)
    (Utilities|FlowControl|Sequence
      (:then_0
        (CallFunction|Paint (Variables|Default|GetCeiling_Top) (Variables|Default|GetBox_Top)))
      (:then_1
        (CallFunction|Paint (Variables|Default|GetCeiling_Bottom) (Variables|Default|GetBox_Bottom))))))

(fn ConstructionScript
  (bind _ceiling_bottom (Variables|Default|GetCeiling_Bottom))
  (bind _ceiling_top (Variables|Default|GetCeiling_Top))
  (Utilities|FlowControl|Sequence
    (:then_0
      (if (Variables|Ceiling|GetTop)
        (Components|StaticMesh|SetStaticMesh _ceiling_top "/Game/RenovationSimulator/Meshes/SM_Ceiling.SM_Ceiling")
        (else
          (Components|StaticMesh|SetStaticMesh _ceiling_top 0))))
    (:then_1
      (if (Variables|Ceiling|GetBottom)
        (Components|StaticMesh|SetStaticMesh _ceiling_bottom "/Game/RenovationSimulator/Meshes/SM_Ceiling.SM_Ceiling")
        (else
          (Components|StaticMesh|SetStaticMesh _ceiling_bottom 0))))))

(fn Paint
  (params (Wall :type Static%20Mesh%20Component%20Object%20Reference) (Collision :type Box%20Component%20Object%20Reference))
  (switch name (Variables|/Game/RenovationSimulator/Demo/Player/FirstPerson/Blueprints/BP_FirstPersonCharacter.BP_FirstPersonCharacter_C|GetPaint_Type (Variables|Player|GetPlayer))
    (:All
      _)
    (:Floor
      _)
    (:Ceiling
      _))
  (if (Collision|IsOverlappingActor Collision (Game|GetPlayerCharacter 0) :!class /Script/Engine.PrimitiveComponent)
    (if (Variables|/Game/RenovationSimulator/Demo/Player/FirstPerson/Blueprints/BP_FirstPersonCharacter.BP_FirstPersonCharacter_C|GetUse_Paint (Variables|Player|GetPlayer))
      (Rendering|Material|SetMaterial Wall 0 (Variables|/Game/RenovationSimulator/Demo/Player/FirstPerson/Blueprints/BP_FirstPersonCharacter.BP_FirstPersonCharacter_C|GetPaint_Current (Variables|Player|GetPlayer)))
      (Default|LevelAddXP (Variables|Player|GetPlayer) 100))))

(fn InterfaceWidgetInput
  (return (Variables|Default|GetWidget)))